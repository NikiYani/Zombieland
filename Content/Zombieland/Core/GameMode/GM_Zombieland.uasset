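; Game mode for Zombieland that runs a survival countdown and decides whether the player wins or loses.
; A looping one-second timer started on BeginPlay decrements GameTime; at zero it clears itself and shows the win widget.
; Otherwise each tick polls the player's HealthComponent and shows a defeat widget on death, without stopping the timer.
; Either outcome switches the player controller to UI-only input with a visible cursor.
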(event `self.ReceiveBeginPlay`
  (bind _returnvalue (`KismetSystemLibrary.K2_SetTimerDelegate` (delegate `CustomEvent`) 1.0 true))
  (set `self.TimerHandle` _returnvalue))

(event `CustomEvent`
  (bind _output_get (set `self.Game Time` (- (`self.Game Time`) 1)))
  (if (== _output_get 0)
    (`KismetSystemLibrary.K2_ClearAndInvalidateTimerHandle` (`self.TimerHandle`))
    (bind _returnvalue (`|CreateWidget` "/Game/Zombieland/Widgets/UI/WBP_Win.WBP_Win_C"))
    (bind _output_get_2 (set `self.WidgetWin` _returnvalue))
    (`UserWidget.AddToViewport` _output_get_2 0)
    (bind _aspc_zombieland (cast `/Game/Zombieland/Core/Controller/PC_Zombieland` (`GameplayStatics.GetPlayerController` 0)))
    (`WidgetBlueprintLibrary.SetInputMode_UIOnlyEx` _aspc_zombieland _output_get_2)
    (set `PlayerController.bShowMouseCursor` true _aspc_zombieland)
    (else
      (bind _asch_player (cast `/Game/Zombieland/Core/Character/CH_Player` (`GameplayStatics.GetPlayerCharacter` 0)))
      (if (`ZLHealthComponent.IsDead` (`ZLDefaultCharacter.HealthComponent` _asch_player))
        (bind _returnvalue_2 (`|CreateWidget` "/Game/Zombieland/Widgets/UI/WBP_Defeat.WBP_Defeat_C"))
        (bind _output_get_3 (set `self.WidgetDefeat` _returnvalue_2))
        (`UserWidget.AddToViewport` _output_get_3 0)
        (bind _aspc_zombieland_2 (cast `/Game/Zombieland/Core/Controller/PC_Zombieland` (`GameplayStatics.GetPlayerController` 0)))
        (`WidgetBlueprintLibrary.SetInputMode_UIOnlyEx` _aspc_zombieland_2 _output_get_3)
        (set `PlayerController.bShowMouseCursor` true _aspc_zombieland_2)))))

(fn `UserConstructionScript`)